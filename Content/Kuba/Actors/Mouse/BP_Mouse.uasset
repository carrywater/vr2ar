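; BP_Mouse is the player character, which moves, melees and collects cheese toward a goal set by Gamemode_Enemy.
; Health calls forward to BPCDamageSystem, whose death, block and damage-response dispatchers drive ragdoll, debug prints and a fall montage.
; Sphere overlaps trigger collection, and AddCheese updates the cheese widget, shown alongside a health bar HUD.
; Hard-coded keys exercise rogue AI noise and damage sensing, passive/attack toggling, and healing.
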(event OnComponentBeginOverlap(Sphere)
  (params (OverlappedComponent :type Primitive%20Component%20Object%20Reference) (OtherActor :type Actor%20Object%20Reference) (OtherComp :type Primitive%20Component%20Object%20Reference) (OtherBodyIndex :type Integer) (bFromSweep :type Boolean) (SweepResult :type Hit%20Result%20Structure%20%28by%20ref%29))
  (Class|BPICollectable|Collect(Message) OtherActor self))

(event Custom|DamageResponse
  (params (DamageResponse :type E_DamageResponse%20Enum :default "NewEnumerator0") (DamageCauser :type Actor%20Object%20Reference))
  ;[1 1 1] Comment
  (Development|PrintString (Utilities|String|EnumtoString DamageResponse))
  (Input|DisableInput 0)
  (Animation|Montage|PlayMontage (Variables|Character|GetMesh) "/Game/Kuba/Actors/Animations/AnimationMontages/COMBAT/FallFlat_UE_Montage.FallFlat_UE_Montage"
    (:OnCompleted
      _)
    (:OnInterrupted
      _))
  (Input|EnableInput (Game|GetPlayerController 0)))

(event Custom|Blocked
  (params (CanBeParried :type Boolean))
  ;[1 1 1] On blocked
  (Development|PrintString "Blocked"))

(event Custom|Death
  (bind _mesh (Variables|Character|GetMesh))
  ;[0.941 0.03594 0.03594] On Death
  (Development|PrintString "Dead")
  (Physics|SetSimulatePhysics _mesh true)
  (Collision|SetCollisionEnabled _mesh "QueryAndPhysics")
  (Input|DisableInput (Game|GetPlayerController 0)))

(event Custom|AddCheese
  (Variables|Default|SetCurrentCheese (+ (Variables|Default|GetCurrentCheese) 1))
  (Rendering|Components|TextRender|SetText (Variables|/Game/Kuba/Cheeze/W_CheezeScore.W_CheezeScore_C|GetCheeseAmount (Variables|Default|GetPlayerCheeseWidgetReference)) (Utilities|Text|FormatText "{Current}/{Max}" (Variables|Default|GetCurrentCheese) (Variables|/Game/Kuba/Gamemode_Enemy.Gamemode_Enemy_C|GetMaxCheeseNeeded (Variables|Default|GetGamemodeReference))))
  (if (>= (Variables|Default|GetCurrentCheese) (Variables|/Game/Kuba/Gamemode_Enemy.Gamemode_Enemy_C|GetMaxCheeseNeeded (Variables|Default|GetGamemodeReference)))
    (Development|PrintString "You have won")))

(event EventBeginPlay
  (Utilities|FlowControl|Sequence
    (:then_0
      (bind _returnvalue (UserInterface|CreateWidget "/Game/Kuba/Cheeze/W_CheezeScore.W_CheezeScore_C"))
      (bind _output_get (Variables|Default|SetPlayerCheeseWidgetReference _returnvalue))
      (UserInterface|Viewport|AddtoViewport _output_get 0)
      (bind _asgamemode_enemy (Utilities|Casting|CastToGamemode_Enemy (Game|GetGameMode)))
      (Variables|Default|SetGamemodeReference _asgamemode_enemy))
    (:then_1
      (bind _returnvalue_2 (UserInterface|CreateWidget "/Game/Kuba/DamageSystem/W_HealthBar_HUD.W_HealthBar_HUD_C" 0 self))
      (bind _output_get_2 (Variables|Default|SetNewVar _returnvalue_2))
      (UserInterface|Viewport|AddtoViewport _output_get_2 0))))

(event Input|ActionEvents|InputActionCrouch
  (params (Key :type Key%20Structure))
  ;[0.0356 0.0356 0.0356] Action Mappings
  (:Pressed
    (Character|Crouch))
  (:Released
    (Character|UnCrouch)))

(event Input|ActionEvents|InputActionJump
  (params (Key :type Key%20Structure))
  ;[0.0356 0.0356 0.0356] Action Mappings
  (:Pressed
    (Character|Jump)))

(event Input|AxisEvents|InputAxisLeftRight
  (params (AxisValue :type Float%20%28single-precision%29))
  ;[0.01938 0.01938 0.01938] Camera Movement
  (Pawn|Input|AddControllerYawInput AxisValue))

(event Input|AxisEvents|InputAxisUpDown
  (params (AxisValue :type Float%20%28single-precision%29))
  ;[0.01938 0.01938 0.01938] Camera Movement
  (Pawn|Input|AddControllerPitchInput AxisValue))

(event Input|AxisEvents|InputAxisForwardBackward
  (params (AxisValue :type Float%20%28single-precision%29))
  ;[0.03071 0.03071 0.03071] Player Movement
  (Pawn|Input|AddMovementInput (Math|Vector|GetForwardVector (Variables|Collision|GetCapsuleComponent)) AxisValue false))

(event Input|AxisEvents|InputAxisWalkLeft
  (params (AxisValue :type Float%20%28single-precision%29))
  ;[0.03071 0.03071 0.03071] Player Movement
  (Pawn|Input|AddMovementInput (Math|Vector|GetRightVector (Variables|Collision|GetCapsuleComponent)) AxisValue false))

(event Input|KeyboardEvents|F
  (params (Key :type Key%20Structure))
  (bind _returnvalue (Transformation|GetActorLocation))
  ;[0.0185 0.01938 0.0185] Create Noise
  (:Pressed
    (Class|Actor|MakeNoise 1.0 self _returnvalue 0.0 "None")
    (Effects|SpawnEmitteratLocation 0 _returnvalue "0, 0, 0" "1.000000,1.000000,1.000000" false)
    (Audio|PlaySoundatLocation "/Engine/VREditor/Sounds/UI/Click_on_Button.Click_on_Button" _returnvalue "0, 0, 0" 1.0 1.0 0.0 0 0 0 0)))

(event Input|KeyboardEvents|X
  (params (Key :type Key%20Structure))
  ;[0.01938 0.01938 0.01938] Report Damage Event
  (:Pressed
    (bind _returnvalue (Actor|GetActorOfClass "/Game/Kuba/Actors/RougeHuman_AI/BP_RougeAI_Base.BP_RougeAI_Base_C"))
    (Class|AISenseDamage|ReportDamageEvent _returnvalue self 0.0 (Transformation|GetActorLocation) "0, 0, 0" "None")))

(event Input|KeyboardEvents|1
  (params (Key :type Key%20Structure))
  ;[0.0356 0.0356 0.0356] Passive/Active State FlipFlop
  (:Pressed
    (bind _returnvalue (Actor|GetActorOfClass "/Game/Kuba/Actors/RougeHuman_AI/BP_RougeAI_Base.BP_RougeAI_Base_C"))
    (bind _asaic_rogue_ai_base (Utilities|Casting|CastToAIC_RogueAI_Base (AI|GetAIController _returnvalue)))
    (Utilities|FlowControl|FlipFlop
      (:A
        (Default|SetStateasPassive _asaic_rogue_ai_base))
      (:B
        (Default|SetStateasAttacking _asaic_rogue_ai_base self false)))))

(event Input|MouseEvents|LeftMouseButton
  (params (Key :type Key%20Structure))
  (bind _returnvalue (Transformation|GetActorLocation))
  ;[1 1 1] Attack
  (:Pressed
    (bind (_outhit _returnvalue_2) (Collision|SphereTraceForObjects _returnvalue (+ _returnvalue (* (Transformation|GetActorForwardVector) 1.2e+02)) 2e+01 (Utilities|Array|MakeArray "ObjectTypeQuery3") false 0 "ForDuration" true "(R=1.000000,G=0.000000,B=0.000000,A=1.000000)" "(R=0.000000,G=1.000000,B=0.000000,A=1.000000)" 1.0))
    (if _returnvalue_2
      (bind _wasdamaged (Class|BPIDamagable|TakeDamage(Message) (.HitActor (Collision|BreakHitResult _outhit)) (Utilities|Struct|MakeS_DamageInfo 1.0 "NewEnumerator2" "NewEnumerator4")))
      (if _wasdamaged
        _
        (else
          _))
      (Audio|PlaySoundatLocation "/Engine/VREditor/Sounds/UI/Dockable_Window_Close.Dockable_Window_Close" (.Location (Collision|BreakHitResult _outhit)) "0, 0, 0" 1.0 1.0 0.0 0 0 0 0)
      (else
        (Audio|PlaySoundatLocation "/Engine/VREditor/Sounds/UI/Teleport_Mode_Entered.Teleport_Mode_Entered" (.Location (Collision|BreakHitResult _outhit)) "0, 0, 0" 1.0 1.0 0.0 0 0 0 0)))))

(event Input|KeyboardEvents|H
  (params (Key :type Key%20Structure))
  ;[1 1 1] Heal
  (:Pressed
    (CallFunction|Heal 1e+01)))

(fn ConstructionScript
  (bind _bpc_damagesystem (Variables|Default|GetBPC_DamageSystem))
  (bind _bpc_damagesystem_2 (Variables|Default|GetBPC_DamageSystem))
  ;[0.03071 0.03071 0.03071] Listening to Event Dispachers
  (EventDispatchers|BindEventtoOnDeath _bpc_damagesystem (EventDispatchers|CreateEvent :!event Custom|Death))
  (EventDispatchers|BindEventtoOnBlocked _bpc_damagesystem (EventDispatchers|CreateEvent :!event Custom|Blocked))
  (EventDispatchers|BindEventtoOnDamageResponse _bpc_damagesystem (EventDispatchers|CreateEvent :!event Custom|DamageResponse))
  (Variables|/Game/Kuba/DamageSystem/BPC_DamageSystem.BPC_DamageSystem_C|SetMaxHealth _bpc_damagesystem_2 1e+02)
  (Variables|/Game/Kuba/DamageSystem/BPC_DamageSystem.BPC_DamageSystem_C|SetHealth _bpc_damagesystem_2 1e+02))

(fn GetCurrentHealth
  (return (Variables|/Game/Kuba/DamageSystem/BPC_DamageSystem.BPC_DamageSystem_C|GetHealth (Variables|Default|GetBPC_DamageSystem))))

(fn GetMaxHealth
  (return (Variables|/Game/Kuba/DamageSystem/BPC_DamageSystem.BPC_DamageSystem_C|GetMaxHealth (Variables|Default|GetBPC_DamageSystem))))

(fn Heal
  (params (Amount :type Float%20%28double-precision%29))
  (bind _newhealth (Default|Heal (Variables|Default|GetBPC_DamageSystem) Amount))
  (return _newhealth))

(fn IsDead
  (return (Variables|/Game/Kuba/DamageSystem/BPC_DamageSystem.BPC_DamageSystem_C|GetIsDead (Variables|Default|GetBPC_DamageSystem))))

(fn TakeDamage
  (params (DamageInfo :type S%20Damage%20Info%20Structure) (Damage%20Causer :type Actor%20Object%20Reference))
  (bind _wasdamaged (Default|TakeDamage (Variables|Default|GetBPC_DamageSystem) DamageInfo Damage%20Causer))
  (return _wasdamaged))